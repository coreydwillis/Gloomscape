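; BP_Gloomi is a roaming, teleporting creature that haunts the level with ambient horror audio.
; A looping timer at a randomly chosen interval moves it to random points within BoundBox, with a teleport sound and delayed, attenuated whispers.
; BeginPlay builds five audio components; player overlap with Sphere plays a random one and removes a separately randomized entry, depleting the pool.
; HitSphere overlap only casts to the player, with no further effect.
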(event OnComponentBeginOverlap(HitSphere)
  (params (OverlappedComponent :type Primitive%20Component%20Object%20Reference) (OtherActor :type Actor%20Object%20Reference) (OtherComp :type Primitive%20Component%20Object%20Reference) (OtherBodyIndex :type Integer) (bFromSweep :type Boolean) (SweepResult :type Hit%20Result%20Structure%20%28by%20ref%29))
  (Utilities|Casting|CastToBP_FirstPersonCharacter OtherActor))

(event OnComponentBeginOverlap(Sphere)
  (params (OverlappedComponent :type Primitive%20Component%20Object%20Reference) (OtherActor :type Actor%20Object%20Reference) (OtherComp :type Primitive%20Component%20Object%20Reference) (OtherBodyIndex :type Integer) (bFromSweep :type Boolean) (SweepResult :type Hit%20Result%20Structure%20%28by%20ref%29))
  (bind _audioarray (Variables|Default|GetAudioArray))
  (bind _returnvalue (Utilities|Array|Length _audioarray))
  (Utilities|Casting|CastToBP_FirstPersonCharacter OtherActor)
  (bind _result (Math|Integer|DecrementInt _returnvalue)
    (:%20%20
      (if (> _returnvalue 0)
        (Audio|Components|Audio|Play (Utilities|Array|Get(acopy) _audioarray (Math|Random|RandomIntegerinRange 0 _result)) 0.0)
        (Utilities|Array|RemoveItem _audioarray (Utilities|Array|Get(acopy) _audioarray (Math|Random|RandomIntegerinRange 0 _result)))))))

(event Custom|MoveAround
  (bind _boundbox (Variables|Default|GetBoundBox))
  (bind (_origin _boxextent) (Collision|GetComponentBounds _boundbox))
  (Audio|PlaySoundatLocation "/Game/Gloomscape/Media/SoundEffects/game-teleport-90735.game-teleport-90735" (Transformation|GetActorLocation) "0, 0, 0" 1.0 1.0 0.0 "/Game/Gloomscape/Media/SoundEffects/gloom_atten.gloom_atten" 0 0 0)
  (Transformation|SetWorldLocation (Variables|Default|GetSharedRoot) (Math|Random|RandomPointinBoundingBox _origin _boxextent) true true)
  (Utilities|FlowControl|Delay (Math|Conversions|ToFloat(Integer) (Math|Random|RandomIntegerinRange 15 60)))
  (bind _returnvalue (Audio|SpawnSoundatLocation "/Game/Gloomscape/Media/SoundEffects/witches-ambient-horror-invented-language-22409.witches-ambient-horror-invented-language-22409" (Transformation|GetActorLocation) "0, 0, 0" 1.0 1.0 0.0 "/Game/Gloomscape/Media/SoundEffects/gloom_atten.gloom_atten" 0))
  (Variables|Default|SetGloomiAudio _returnvalue))

(event Custom|CreateSoundEffectArray
  (bind _returnvalue (AddComponent|AddAudioComponent false))
  (bind _returnvalue_2 (AddComponent|AddAudioComponent false))
  (bind _returnvalue_3 (AddComponent|AddAudioComponent false))
  (bind _returnvalue_4 (AddComponent|AddAudioComponent false))
  (bind _returnvalue_5 (AddComponent|AddAudioComponent false))
  (Variables|Default|SetAudioArray (Utilities|Array|MakeArray _returnvalue _returnvalue_2 _returnvalue_3 _returnvalue_4 _returnvalue_5)))

(event EventBeginPlay
  (CallFunction|CreateSoundEffectArray)
  (Utilities|Time|SetTimerbyEvent (delegate Custom|MoveAround) (Math|Conversions|ToFloat(Integer) (Math|Random|RandomIntegerinRange 10 20)) true)
  (Utilities|FlowControl|Delay (Math|Conversions|ToFloat(Integer) (Math|Random|RandomIntegerinRange 15 60)))
  (bind _returnvalue (Audio|SpawnSoundatLocation "/Game/Gloomscape/Media/SoundEffects/witches-ambient-horror-invented-language-22409.witches-ambient-horror-invented-language-22409" (Transformation|GetActorLocation) "0, 0, 0" 1.0 1.0 0.0 "/Game/Gloomscape/Media/SoundEffects/gloom_atten.gloom_atten" 0))
  (Variables|Default|SetGloomiAudio _returnvalue))

(fn ConstructionScript)