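; BP_GloomGameMode is the Gloomscape game mode, with an unfinished or disabled wolf population cap.
; On BeginPlay it gathers all BP_WolfCharacterNew actors and casts the game state to BP_GloomGameState, then does nothing further.
; Disconnected logic would shuffle the wolves, destroy random extras beyond the game state's WolfPopTotal, and track WolvesTotal and WolvesLeft, but it never runs.
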(event EventBeginPlay
  (bind _outactors (Actor|GetAllActorsOfClass "/Game/Gloomscape/Blueprints/BP_WolfCharacterNew.BP_WolfCharacterNew_C"))
  (bind _asbp_gloom_game_state (Utilities|Casting|CastToBP_GloomGameState (Game|GetGameState))))

(fn ConstructionScript)