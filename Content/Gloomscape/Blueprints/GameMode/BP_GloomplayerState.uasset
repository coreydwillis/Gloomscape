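; Player state for Gloomscape that tracks collected gloomspheres and controls temporary shifts in the Gloom fog.
; On BeginPlay it creates the sphere counter widget and stores the default fog color; each pickup increments the count and updates the widget.
; ChangeGloom finds the BP_TheGloom actor, sets height falloff and adjusts density, adding fog instead when density would reach zero or below.
; It flashes the fog albedo to the given color, restoring the default after a second.
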(event EventBeginPlay
  (bind _returnvalue (UserInterface|CreateWidget "/Game/Gloomscape/Blueprints/UI/WBP_Gloomspheres.WBP_Gloomspheres_C"))
  (bind _output_get (Variables|Default|SetGloomsphereBP _returnvalue))
  (UserInterface|Viewport|AddtoViewport _output_get 0)
  (Variables|Default|SetGloom%20Color (Math|Color|MakeColor 194 108 68)))

(event EventChangeGloom
  (params (Color :type Color%20Structure) (Intensity :type Float%20%28double-precision%29))
  (bind _asbp_the_gloom (Utilities|Casting|CastToBP_TheGloomClass "/Game/Gloomscape/Blueprints/BP_TheGloom.BP_TheGloom_C"))
  (bind _returnvalue (Actor|GetActorOfClass _asbp_the_gloom))
  (Class|ExponentialHeightFogComponent|SetFogHeightFalloff (Variables|/Game/Gloomscape/Blueprints/BP_TheGloom.BP_TheGloom_C|GetExponentialHeightFog _returnvalue) 1.5)
  (if (<= (+ (Variables|/Script/Engine.ExponentialHeightFogComponent|GetFogDensity (Variables|/Game/Gloomscape/Blueprints/BP_TheGloom.BP_TheGloom_C|GetExponentialHeightFog _returnvalue)) Intensity) 0.0)
    (Class|ExponentialHeightFogComponent|SetFogDensity (Variables|/Game/Gloomscape/Blueprints/BP_TheGloom.BP_TheGloom_C|GetExponentialHeightFog _returnvalue) (+ (Variables|/Script/Engine.ExponentialHeightFogComponent|GetFogDensity (Variables|/Game/Gloomscape/Blueprints/BP_TheGloom.BP_TheGloom_C|GetExponentialHeightFog _returnvalue)) 0.25))
    (else
      (Class|ExponentialHeightFogComponent|SetFogDensity (Variables|/Game/Gloomscape/Blueprints/BP_TheGloom.BP_TheGloom_C|GetExponentialHeightFog _returnvalue) (+ (Variables|/Script/Engine.ExponentialHeightFogComponent|GetFogDensity (Variables|/Game/Gloomscape/Blueprints/BP_TheGloom.BP_TheGloom_C|GetExponentialHeightFog _returnvalue)) Intensity))))
  (Class|ExponentialHeightFogComponent|SetVolumetricFogAlbedo (Variables|/Game/Gloomscape/Blueprints/BP_TheGloom.BP_TheGloom_C|GetExponentialHeightFog _returnvalue) Color)
  (Utilities|FlowControl|Delay 1.0)
  (Class|ExponentialHeightFogComponent|SetVolumetricFogAlbedo (Variables|/Game/Gloomscape/Blueprints/BP_TheGloom.BP_TheGloom_C|GetExponentialHeightFog _returnvalue) (Variables|Default|GetGloom%20Color)))

(event EventPickupSqhere
  (bind _output_get (Variables|Default|SetCurrentGloomSqheres (Variables|Default|GetCurrentGloomSqheres)))
  (bind _result (Math|Integer|IncrementInt _output_get)
    (:%20%20
      (Class|BPIGloomsqhereUI|UpdateSphereCount(Message) (Variables|Default|GetGloomsphereBP) _result))))

(fn ConstructionScript)