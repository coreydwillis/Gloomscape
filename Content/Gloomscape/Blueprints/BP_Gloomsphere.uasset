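; BP_Gloomsphere is a collectible sphere actor that the first-person player picks up by touching it.
; On BeginPlay it adds an audio component, then starts that sound playing after a delay.
; Overlap with BP_FirstPersonCharacter plays an attenuated gong at the sphere's location, calls the pickup message on the player state, stops the sphere's audio and destroys the actor.
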(event OnComponentBeginOverlap(Sphere)
  (params (OverlappedComponent :type Primitive%20Component%20Object%20Reference) (OtherActor :type Actor%20Object%20Reference) (OtherComp :type Primitive%20Component%20Object%20Reference) (OtherBodyIndex :type Integer) (bFromSweep :type Boolean) (SweepResult :type Hit%20Result%20Structure%20%28by%20ref%29))
  (Utilities|Casting|CastToBP_FirstPersonCharacter OtherActor)
  (Audio|PlaySoundatLocation "/Game/Gloomscape/Media/SoundEffects/gong.gong" (Transformation|GetActorLocation) "0, 0, 0" 1.0 1.0 0.0 "/Game/Gloomscape/Media/SoundEffects/gloom_atten.gloom_atten" 0 0 0)
  (Class|BPIGloomsqherePickup|PickupSqhere(Message) (Game|GetPlayerState 0))
  (bind _output_get (Variables|Default|SetGloomsphere (Variables|Default|GetGloomsphere)))
  (Audio|Components|Audio|Stop _output_get)
  (Actor|DestroyActor))

(event EventBeginPlay
  (bind _returnvalue (AddComponent|AddAudioComponent false))
  (bind _output_get (Variables|Default|SetGloomsphere _returnvalue))
  (Utilities|FlowControl|Delay 1e+01)
  (Audio|Components|Audio|Play _output_get 0.0))

(fn ConstructionScript)