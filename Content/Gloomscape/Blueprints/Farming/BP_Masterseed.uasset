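; BP_Masterseed is a farming seed actor, apparently a base for crop types, that visually grows over four days.
; Each NewDayGrow event increments an internal day counter, capped at four, then waits briefly before triggering the matching growth stage event.
; Each stage event swaps the static mesh to that stage's mesh variable.
; The Plant function takes a player and is a stub that always returns false.
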(event Custom|Forth%20Growth%20Stage
  (Components|StaticMesh|SetStaticMesh (Variables|Default|GetStaticMesh) (Variables|Default|GetForth%20Growth%20Stage%20Mesh)))

(event Custom|Third%20Growth%20Stage
  (Components|StaticMesh|SetStaticMesh (Variables|Default|GetStaticMesh) (Variables|Default|GetThird%20Growth%20Stage%20Mesh)))

(event Custom|Second%20Growth%20Stage
  (Components|StaticMesh|SetStaticMesh (Variables|Default|GetStaticMesh) (Variables|Default|GetSecond%20Growth%20Stage%20Mesh)))

(event Custom|First%20Growth%20Stage
  (Components|StaticMesh|SetStaticMesh (Variables|Default|GetStaticMesh) (Variables|Default|GetFirstGrowthStageMeth)))

(event EventNewDayGrow
  (if (< (Variables|Default|GetInternalDayCounter) 4)
    (bind _result (Math|Integer|IncrementInt (Variables|Default|GetInternalDayCounter))
      (:%20%20
        (Variables|Default|SetInternalDayCounter _result)
        (Utilities|FlowControl|Delay 1.0)
        (switch int (Variables|Default|GetInternalDayCounter)
          (:1
            (CallFunction|FirstGrowthStage))
          (:2
            (CallFunction|SecondGrowthStage))
          (:3
            (CallFunction|ThirdGrowthStage))
          (:4
            (CallFunction|ForthGrowthStage)))))))

(fn ConstructionScript)

(fn Plant
  (params (Player :type BP%20First%20Person%20Character%20Object%20Reference))
  (return false))