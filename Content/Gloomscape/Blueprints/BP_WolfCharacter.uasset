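; BP_WolfCharacter is an enemy wolf that roams randomly, chases the first-person player and bites to drain health.
; Roaming repeats AIMoveTo to random reachable points with random pauses.
; Sphere overlap snarls and starts a self-repeating chase, and leaving it resumes roaming.
; Bite overlap starts a delayed attack loop that decrements health in BP_GloomGameState, updates its UI, plays bite animation and sound, and triggers the death message at zero.
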(event OnComponentBeginOverlap(Sphere)
  (params (OverlappedComponent :type Primitive%20Component%20Object%20Reference) (OtherActor :type Actor%20Object%20Reference) (OtherComp :type Primitive%20Component%20Object%20Reference) (OtherBodyIndex :type Integer) (bFromSweep :type Boolean) (SweepResult :type Hit%20Result%20Structure%20%28by%20ref%29))
  (Utilities|Casting|CastToBP_FirstPersonCharacter OtherActor)
  (Variables|Default|SetIs%20Chasing%20Player true)
  (Audio|PlaySoundatLocation "/Game/Gloomscape/Media/SoundEffects/beast-snarling-82801.beast-snarling-82801" (Transformation|GetActorLocation) "0, 0, 0" 5.0 0.8 0.0 0 0 0 0)
  (CallFunction|ChasePlayer))

(event OnComponentEndOverlap(Sphere)
  (params (OverlappedComponent :type Primitive%20Component%20Object%20Reference) (OtherActor :type Actor%20Object%20Reference) (OtherComp :type Primitive%20Component%20Object%20Reference) (OtherBodyIndex :type Integer))
  (Utilities|Casting|CastToBP_FirstPersonCharacter OtherActor)
  (Variables|Default|SetIs%20Chasing%20Player false)
  (CallFunction|RandomRoam))

(event OnComponentBeginOverlap(Bite)
  (params (OverlappedComponent :type Primitive%20Component%20Object%20Reference) (OtherActor :type Actor%20Object%20Reference) (OtherComp :type Primitive%20Component%20Object%20Reference) (OtherBodyIndex :type Integer) (bFromSweep :type Boolean) (SweepResult :type Hit%20Result%20Structure%20%28by%20ref%29))
  (Utilities|Casting|CastToBP_FirstPersonCharacter OtherActor)
  (Variables|Default|SetIn%20Biting%20Range true)
  (CallFunction|WolfAttack))

(event OnComponentEndOverlap(Bite)
  (params (OverlappedComponent :type Primitive%20Component%20Object%20Reference) (OtherActor :type Actor%20Object%20Reference) (OtherComp :type Primitive%20Component%20Object%20Reference) (OtherBodyIndex :type Integer))
  (Utilities|Casting|CastToBP_FirstPersonCharacter OtherActor)
  (Variables|Default|SetIn%20Biting%20Range false)
  (CallFunction|ChasePlayer))

(event Custom|Random%20Roam
  (AI|AIMoveTo self (.RandomLocation (AI|Navigation|GetRandomReachablePointinRadius (Transformation|GetActorLocation) 3e+03 0 0)) 0 5.0 false
    (:OnSuccess
      (if (not (Variables|Default|GetIs%20Chasing%20Player))
        (Utilities|FlowControl|Delay (Math|Random|RandomFloatinRange 0.01 1e+01))
        (CallFunction|RandomRoam)))))

(event Custom|Chase%20Player
  (AI|AIMoveTo self "0, 0, 0" (stale OnComponentBeginOverlap(Sphere) OtherActor) 5.0 false
    (:OnSuccess
      (if (Variables|Default|GetIs%20Chasing%20Player)
        (CallFunction|ChasePlayer)
        (else
          (CallFunction|RandomRoam))))))

(event Custom|WolfAttack
  (params (Victim :type Actor%20Object%20Reference))
  (bind _asbp_gloom_game_state (Utilities|Casting|CastToBP_GloomGameState (Game|GetGameState)))
  (bind _result (Math|Integer|DecrementInt (Variables|/Game/Gloomscape/Blueprints/GameMode/BP_GloomGameState.BP_GloomGameState_C|GetPlayerHealthCurrent _asbp_gloom_game_state))
    (:%20%20
      (bind _output_get (Variables|/Game/Gloomscape/Blueprints/GameMode/BP_GloomGameState.BP_GloomGameState_C|SetPlayerHealthCurrent _asbp_gloom_game_state _result))
      (Class|BPIPlayerUI|UpdatePlayerHealth(Message) (Variables|/Game/Gloomscape/Blueprints/GameMode/BP_GloomGameState.BP_GloomGameState_C|GetPlayerUI _asbp_gloom_game_state) _output_get)
      (if (> _output_get 0)
        (Components|Animation|PlayAnimation (Variables|Character|GetMesh) "/Game/AnimalVarietyPack/Wolf/Animations/ANIM_Wolf_Bite.ANIM_Wolf_Bite" false)
        (Audio|PlaySoundatLocation "/Game/Gloomscape/Media/SoundEffects/bone-crunch-fast-105708.bone-crunch-fast-105708" (Transformation|GetActorLocation) "0, 0, 0" 1.0 1.0 0.0 0 0 0 0)
        (Utilities|FlowControl|Delay 2.0)
        (Components|Animation|SetAnimationMode (Variables|Character|GetMesh) "AnimationBlueprint")
        (if (Variables|Default|GetIn%20Biting%20Range)
          (Utilities|FlowControl|Delay 2.0)
          (CallFunction|WolfAttack Victim)
          (else
            (CallFunction|RandomRoam)))
        (else
          (Class|BPIGameStates|PlayerDead(Message) _asbp_gloom_game_state))))))

(event EventBeginPlay
  (Utilities|FlowControl|Delay (Math|Random|RandomFloatinRange 1.0 6.0))
  (CallFunction|RandomRoam))

(fn ConstructionScript)