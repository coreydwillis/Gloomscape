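; BP_Gloomgate is a level exit gate that sends the player to GloomLevel2 once enough gloom spheres are collected.
; It plays an attenuated looping-style gate sound at its location on BeginPlay.
; When the first-person character overlaps its box, it checks the sphere count in the player state.
; With enough spheres it plays a travel sound and opens the level after a delay, otherwise it shows a collect-more widget with an error sound.
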(event OnComponentBeginOverlap(Box)
  (params (OverlappedComponent :type Primitive%20Component%20Object%20Reference) (OtherActor :type Actor%20Object%20Reference) (OtherComp :type Primitive%20Component%20Object%20Reference) (OtherBodyIndex :type Integer) (bFromSweep :type Boolean) (SweepResult :type Hit%20Result%20Structure%20%28by%20ref%29))
  (Utilities|Casting|CastToBP_FirstPersonCharacter OtherActor)
  (bind _asbp_gloomplayer_state (Utilities|Casting|CastToBP_GloomplayerState (Game|GetPlayerState 0)))
  (if (>= (Variables|/Game/Gloomscape/Blueprints/GameMode/BP_GloomplayerState.BP_GloomplayerState_C|GetCurrentGloomSqheres _asbp_gloomplayer_state) 5)
    (Audio|PlaySound2D "/Game/Gloomscape/Media/SoundEffects/time-travel-83472.time-travel-83472" 1.0 1.0 0.0 0 0)
    (Utilities|FlowControl|Delay 2.5)
    (Game|OpenLevel(byName) "GloomLevel2")
    (else
      (bind _returnvalue (UserInterface|CreateWidget "/Game/Gloomscape/Blueprints/UI/WBP_CollectMore.WBP_CollectMore_C"))
      (UserInterface|Viewport|AddtoViewport _returnvalue 0)
      (Audio|PlaySound2D "/Game/Gloomscape/Media/SoundEffects/wrong-47985.wrong-47985" 1.0 1.0 0.0 0 0))))

(event EventBeginPlay
  (bind _returnvalue (Audio|SpawnSoundatLocation "/Game/Gloomscape/Media/SoundEffects/gloomgate.gloomgate" (Transformation|GetActorLocation) "0, 0, 0" 1.0 1.0 0.0 "/Game/Gloomscape/Media/SoundEffects/gloomGate_atten.gloomGate_atten" 0 false))
  (Variables|Default|SetGloomGateSound _returnvalue))

(fn ConstructionScript)