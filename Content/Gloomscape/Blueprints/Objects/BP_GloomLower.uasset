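; BP_GloomLower is an interactable object that lets the player lower gloom with the interact input.
; Its capsule overlap events set an Overlapping flag and show or clear a "Press E to Lower Gloom" prompt through BP_GloomplayerState, without filtering the overlapping actor.
; While Overlapping is set, each IA_InteractBTN trigger sends a gloom change message with a color and negative intensity to the first player's state.
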(event OnComponentBeginOverlap(Capsule)
  (params (OverlappedComponent :type Primitive%20Component%20Object%20Reference) (OtherActor :type Actor%20Object%20Reference) (OtherComp :type Primitive%20Component%20Object%20Reference) (OtherBodyIndex :type Integer) (bFromSweep :type Boolean) (SweepResult :type Hit%20Result%20Structure%20%28by%20ref%29))
  (bind _output_get (Variables|Default|SetOverlapping true))
  (bind _asbp_gloomplayer_state (Utilities|Casting|CastToBP_GloomplayerState (Game|GetPlayerState 0)))
  (Class|BPIChangeGloom|InteractUI(Message) _asbp_gloomplayer_state _output_get (Utilities|Text|MakeLiteralText "Press E to Lower Gloom")))

(event OnComponentEndOverlap(Capsule)
  (params (OverlappedComponent :type Primitive%20Component%20Object%20Reference) (OtherActor :type Actor%20Object%20Reference) (OtherComp :type Primitive%20Component%20Object%20Reference) (OtherBodyIndex :type Integer))
  (bind _output_get (Variables|Default|SetOverlapping false))
  (bind _asbp_gloomplayer_state (Utilities|Casting|CastToBP_GloomplayerState (Game|GetPlayerState 0)))
  (Class|BPIChangeGloom|InteractUI(Message) _asbp_gloomplayer_state _output_get))

(event Input|EnhancedActionEvents|EnhancedInputActionIA_InteractBTN
  (params (ActionValue :type Boolean) (ElapsedSeconds :type Float%20%28double-precision%29) (TriggeredSeconds :type Float%20%28double-precision%29) (InputAction :type Input%20Action%20Object%20Reference :default "/Game/Gloomscape/FirstPerson/Input/Actions/IA_InteractBTN.IA_InteractBTN"))
  (:Triggered
    (if (Variables|Default|GetOverlapping)
      (bind _asbp_gloomplayer_state (Utilities|Casting|CastToBP_GloomplayerState (Game|GetPlayerState 0)))
      (Class|BPIChangeGloom|ChangeGloom(Message) _asbp_gloomplayer_state (Math|Color|MakeColor 68 159 68) -0.25))))

(event EventBeginPlay)

(fn ConstructionScript)